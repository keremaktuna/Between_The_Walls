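; Main menu player controller that gathers the local player's identity for the game.
; Shortly after BeginPlay it reads the Steam persona name and avatar into PlayerInfo, continuing even if the avatar fetch fails, then messages the game instance to save it and handle main menu player info.
; Without Steam it only sets PlayerName from the platform user name.
; The A key prints the stored name.
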(event `self.ReceiveBeginPlay`
  (bind _returnvalue (`GameplayStatics.GetGameInstance`))
  (`KismetSystemLibrary.Delay` 0.2)
  (if (`AdvancedSessionsLibrary.HasOnlineSubsystem` "steam")
    (bind _returnvalue_2 (`AdvancedSteamFriendsLibrary.GetSteamPersonaName` (`AdvancedSessionsLibrary.GetUniqueNetID` self)))
    (set `self.PlayerName` (`KismetTextLibrary.Conv_StringToText` _returnvalue_2))
    (bind _returnvalue_3 (`AdvancedSteamFriendsLibrary.GetSteamFriendAvatar` (`AdvancedSessionsLibrary.GetUniqueNetID` self))
      (:`OnSuccess`
        _)
      (:`OnFailure`
        _))
    (bind _structout (setmembers `/Game/_Main/S_PlayerInfo` :`StructRef` (`self.PlayerInfo`) :`PlayerName` (`self.PlayerName`) :`PlayerImage` _returnvalue_3))
    (message `/Game/_Main/BPI_GameInstance.SavePlayerInfo` _returnvalue _structout)
    (message `/Game/_Main/BPI_GameInstance.MainMenuPlayerInfo` _returnvalue)
    (else
      (set `self.PlayerName` (`KismetTextLibrary.Conv_StringToText` (`KismetSystemLibrary.GetPlatformUserName`))))))

(event `Key|A`
  (params (Key :type "Key Structure"))
  (:`Pressed`
    (`KismetSystemLibrary.PrintText` (`.PlayerName_11_70EDE7CF468A2F722554A5A5B05F298B` (break `/Game/_Main/S_PlayerInfo` (`self.PlayerInfo`))))))

(fn `UserConstructionScript`)